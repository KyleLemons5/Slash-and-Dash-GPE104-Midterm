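; Player dash ability with limited, recharging charges, triggered by F or Left Shift and shown on a DashHud widget that starts hidden.
; A dash follows held WASD keys (forward by default), overriding pawn velocity each frame while making the player invincible, then drops to max movement speed.
; Each finished dash calls RechargeDash, which refills charges one by one and updates the HUD.
; Both timed phases use a Delay-based while-loop macro instead of Tick.
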(event `self.ReceiveBeginPlay`
  (bind _dashhudcache (`self.DashHudCache`))
  (set `self.Dashes` (`self.MaxDashes`))
  (bind _returnvalue (`|CreateWidget` "/Game/UIStuff/DashHud.DashHud_C" (`GameplayStatics.GetPlayerController` 0)))
  (bind _output_get (set `self.DashHudCache` _returnvalue))
  (`UserWidget.AddToViewport` _output_get 0)
  (`/Game/UIStuff/DashHud.UpdateDashBar` _dashhudcache (`self.Dashes`) (`self.DashChargeTime`) (`self.ChargeTime`))
  (`Widget.SetVisibility` _dashhudcache "Hidden"))

(event `Key|F`
  (params (Key :type "Key Structure"))
  (bind _returnvalue (`Pawn.GetMovementComponent` (`GameplayStatics.GetPlayerPawn` 0)))
  (:`Pressed`
    (if (>= (`self.Dashes`) 1) :!label _label
      (bind _output_get (set `self.Dashes` (- (`self.Dashes`) 1)))
      (`/Game/UIStuff/DashHud.UpdateDashBar` (`self.DashHudCache`) _output_get (`self.DashChargeTime`) 0.0)
      (`GameplayStatics.PlaySoundAtLocation` "/Game/SoundEffects/whoosh-6316.whoosh-6316" (`Actor.K2_GetActorLocation` (`GameplayStatics.GetPlayerCharacter` 0)) (struct) 1.0 1.0 0.0 null null null null)
      (`self.CalculateDashDirection`)
      (bind _asbp_first_person_character (cast `/Game/FirstPerson/Blueprints/BP_FirstPersonCharacter` (`GameplayStatics.GetPlayerCharacter` 0)))
      (set `/Game/Blueprints/PlayerHealth.IsInvincible` true (`/Game/FirstPerson/Blueprints/BP_FirstPersonCharacter.PlayerHealth` _asbp_first_person_character))
      (set `self.Time` 0.0)
      (`self.DelayedWhileLoop` (>= (`self.DashTime`) (`self.Time`))
        (:`Loop Body`
          (set `MovementComponent.Velocity` (`self.DashDirection`) _returnvalue)
          (set `self.Time` (+ (`self.Time`) (`GameplayStatics.GetWorldDeltaSeconds`))))
        (:`Completed`
          (set `MovementComponent.Velocity` (* (`KismetMathLibrary.Normal` (`self.DashDirection`)) (`MovementComponent.GetMaxSpeed` _returnvalue)) _returnvalue)
          (`self.RechargeDash`)
          (bind _asbp_first_person_character_2 (cast `/Game/FirstPerson/Blueprints/BP_FirstPersonCharacter` (`GameplayStatics.GetPlayerCharacter` 0)))
          (set `/Game/Blueprints/PlayerHealth.IsInvincible` false (`/Game/FirstPerson/Blueprints/BP_FirstPersonCharacter.PlayerHealth` _asbp_first_person_character_2)))))))

(event `Key|LeftShift`
  (params (Key :type "Key Structure"))
  (:`Pressed`
    (goto _label)))

(event `RechargeDash`
  (if (>= (`self.ChargeTime`) (`self.DashChargeTime`))
    (set `self.ChargeTime` 0.0))
  (`self.DelayedWhileLoop` (>= (`self.DashChargeTime`) (`self.ChargeTime`))
    (:`Loop Body`
      (set `self.ChargeTime` (+ (`self.ChargeTime`) (`GameplayStatics.GetWorldDeltaSeconds`)))
      (`/Game/UIStuff/DashHud.UpdateDashBar` (`self.DashHudCache`) (`self.Dashes`) (`self.DashChargeTime`) (`self.ChargeTime`)))
    (:`Completed`
      (set `self.Dashes` (`KismetMathLibrary.Clamp` (+ (`self.Dashes`) 1) 0 (`self.MaxDashes`)))
      (if (< (`self.Dashes`) (`self.MaxDashes`))
        (`self.RechargeDash`)))))

(fn `CalculateDashDirection`
  (returns (DashDirection :type "Vector Structure"))
  (bind _returnvalue (`GameplayStatics.GetPlayerController` 0))
  (bind _returnvalue_2 (`Actor.K2_GetActorRotation` (`GameplayStatics.GetPlayerPawn` 0)))
  (bind _returnvalue_3 (`KismetMathLibrary.GetRightVector` _returnvalue_2))
  (bind _returnvalue_4 (`KismetMathLibrary.Conv_RotatorToVector` _returnvalue_2))
  (set `self.DashDirection` (0.0 0.0 0.0))
  (if (`PlayerController.IsInputKeyDown` _returnvalue "W")
    (set `self.DashDirection` (+ (`self.DashDirection`) _returnvalue_4)))
  (if (`PlayerController.IsInputKeyDown` _returnvalue "S")
    (set `self.DashDirection` (+ (`self.DashDirection`) (* _returnvalue_4 (-1.0 -1.0 0.0)))))
  (if (`PlayerController.IsInputKeyDown` _returnvalue "D")
    (set `self.DashDirection` (+ (`self.DashDirection`) _returnvalue_3)))
  (if (`PlayerController.IsInputKeyDown` _returnvalue "A")
    (bind _output_get (set `self.DashDirection` (+ (`self.DashDirection`) (* _returnvalue_3 (-1.0 -1.0 0.0))))))
  (bind _output_get_2 (set `self.DashDirection` (* (`KismetMathLibrary.Normal` _output_get) (`self.DashSpeed`))))
  (bind (_x _y) (`KismetMathLibrary.BreakVector3f` _output_get_2))
  (if (and (== _x 0.0) (== _y 0.0))
    (set `self.DashDirection` (* (* (`KismetMathLibrary.Normal` (`KismetMathLibrary.Conv_RotatorToVector` (`Actor.K2_GetActorRotation` (`GameplayStatics.GetPlayerPawn` 0)))) (1.0 1.0 0.0)) (`self.DashSpeed`))))
  (return (`self.DashDirection`)))