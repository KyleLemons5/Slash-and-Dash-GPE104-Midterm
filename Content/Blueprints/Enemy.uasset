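; Stationary-logic shooter enemy that fires projectiles at the first-person player while they overlap it and awards points when destroyed.
; BeginPlay scales the detection sphere by its radius; player overlap starts a looping SpawnProjectile timer, offset to fire immediately, and end overlap clears it.
; Each shot spawns at the Sphere component with the player pawn as Instigator, then gets a velocity impulse toward the player's current position.
; On destruction, its Points go to SlashAndDashInstance.
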(event `self.ReceiveBeginPlay`
  (bind _detection_radius (`self.Detection Radius`))
  (`SceneComponent.SetWorldScale3D` (`self.Detection Sphere`) (`KismetMathLibrary.MakeVector` _detection_radius _detection_radius _detection_radius)))

(event `self.ReceiveActorBeginOverlap`
  (params (OtherActor :type "Actor Object Reference"))
  (bind _shot_delay (`self.Shot Delay`))
  (cast `/Game/FirstPerson/Blueprints/BP_FirstPersonCharacter` OtherActor)
  (bind _returnvalue (`KismetSystemLibrary.K2_SetTimer` null "SpawnProjectile" _shot_delay true (* _shot_delay -1.0)))
  (set `self.SpawnProjectileTimer` _returnvalue))

(event `self.ReceiveActorEndOverlap`
  (params (OtherActor :type "Actor Object Reference"))
  (cast `/Game/FirstPerson/Blueprints/BP_FirstPersonCharacter` OtherActor)
  (`KismetSystemLibrary.K2_ClearAndInvalidateTimerHandle` (`self.SpawnProjectileTimer`)))

(event `self.ReceiveDestroyed`
  (bind _asslash_and_dash_instance (cast `/Game/Blueprints/SlashAndDashInstance` (`GameplayStatics.GetGameInstance`)))
  (`/Game/Blueprints/SlashAndDashInstance.AddPoints` _asslash_and_dash_instance (`self.Points`)))

(fn `SpawnProjectile`
  (bind _returnvalue (`|SpawnActorFromClass` "/Game/Blueprints/Projectile.Projectile_C" (`KismetMathLibrary.MakeTransform` (`SceneComponent.K2_GetComponentLocation` (`self.Sphere`))) "AlwaysSpawn" "MultiplyWithRoot" null (`GameplayStatics.GetPlayerPawn` 0)))
  (`PrimitiveComponent.AddImpulse` (`/Game/Blueprints/Projectile.ProjectileSphere` _returnvalue) (* (`KismetMathLibrary.Normal` (- (`self.K2_GetActorLocation` (`GameplayStatics.GetPlayerCharacter` 0)) (`SceneComponent.K2_GetComponentLocation` (`self.Sphere`)))) (`self.ProjectileSpeed`)) "None" true))

(fn `UserConstructionScript`)