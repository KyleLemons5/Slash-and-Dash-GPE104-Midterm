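; EnemyHealth is a health Blueprint for enemies that tracks damage and destroys its owning actor when health runs out.
; It sets Health to MaxHealth on BeginPlay, and TakeDamage subtracts incoming damage from it.
; A non-lethal hit plays a metal footstep sound at the owner's location.
; At zero or below, Death plays a louder sword-hit sound there and destroys the owner.
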(event `self.ReceiveBeginPlay`
  (set `self.Health` (`self.MaxHealth`)))

(fn `Death`
  (`GameplayStatics.PlaySoundAtLocation` "/Game/SoundEffects/hit-swing-sword-small-2-95566.hit-swing-sword-small-2-95566" (`Actor.K2_GetActorLocation` (`self.GetOwner`)) (struct) 2.5 1.0 0.0 null null null null)
  (`Actor.K2_DestroyActor` (`self.GetOwner`)))

(fn `takeDamage`
  (params (Damage :type "Float (double-precision)"))
  (bind _output_get (set `self.Health` (- (`self.Health`) Damage)))
  (if (<= _output_get 0.0)
    (`self.Death`)
    (else
      (`GameplayStatics.PlaySoundAtLocation` "/Game/SoulCity/Sound/Wav/Footstep_Metal01.Footstep_Metal01" (`Actor.K2_GetActorLocation` (`self.GetOwner`)) (struct) 1.0 1.0 0.0 null null null null))))