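; PlayerHealth tracks the player's health, applying damage and healing and showing the result on a HealthHud widget.
; BeginPlay fills health and creates the widget hidden; any later health update makes it visible and refreshes it.
; TakeDamage is skipped while invincible and, at zero or below, hands death to the SlashAndDashInstance game instance.
; DoHeal clamps health between zero and the maximum.
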(event `self.ReceiveBeginPlay`
  (set `self.Health` (`self.MaxHealth`))
  (bind _returnvalue (`|CreateWidget` "/Game/UIStuff/HealthHud.HealthHud_C" (`GameplayStatics.GetPlayerController` 0)))
  (bind _output_get (set `self.Healthbar Cache` _returnvalue))
  (`UserWidget.AddToViewport` _output_get 0)
  (`self.updateUI`)
  (`Widget.SetVisibility` (`self.Healthbar Cache`) "Hidden"))

(fn `Death`
  (bind _asslash_and_dash_instance (cast `/Game/Blueprints/SlashAndDashInstance` (`GameplayStatics.GetGameInstance`)))
  (`/Game/Blueprints/SlashAndDashInstance.Death` _asslash_and_dash_instance))

(fn `doHeal`
  (params (Heal :type "Float (double-precision)"))
  (set `self.Health` (`KismetMathLibrary.FClamp` (+ Heal (`self.Health`)) 0.0 (`self.MaxHealth`)))
  (`self.updateUI`))

(fn `takeDamage`
  (params (Damage :type "Float (double-precision)"))
  (if (not (`self.IsInvincible`))
    (bind _output_get (set `self.Health` (- (`self.Health`) Damage)))
    (`self.updateUI`)
    (if (<= _output_get 0.0)
      (`self.Death`))))

(fn `updateUI`
  (bind _healthbar_cache (`self.Healthbar Cache`))
  (if (not (`Widget.IsVisible` _healthbar_cache))
    (`Widget.SetVisibility` _healthbar_cache "Visible"))
  (`/Game/UIStuff/HealthHud.UpdateHealth` (`self.Healthbar Cache`) (`self.Health`) (`self.MaxHealth`)))