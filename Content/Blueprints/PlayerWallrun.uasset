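; Player wallrun logic: holding D or A while falling beside a steep wall runs along it, with W/S choosing direction.
; A looping timer line-traces to the sides, then uses LaunchCharacter to stick and move the player while easing gravity toward a target.
; A delayed-loop macro limits run time, and ending a run restores gravity and starts a cooldown that landing clears.
; Space jumps off along the wall normal, and Tick rolls the camera during runs.
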(event `Start`
  (params (`Character Movement Component` :type "CharacterMovementComponent Object Reference"))
  (bind _output_get (set `self.Movement Component` `Character Movement Component`))
  (set `self.DefaultGravity` (`CharacterMovementComponent.GravityScale` _output_get))
  (`KismetSystemLibrary.K2_SetTimer` null "Wallrun Update" 0.02 true))

(event `Key|SpaceBar`
  (params (Key :type "Key Structure"))
  (:`Pressed`
    (if (`self.Is Wallrunning`)
      (`self.Wallrun Jump`))))

(event `Land`
  (`self.Wallrun End`)
  (set `self.Wallrun Enabled` true))

(event `self.ReceiveTick`
  (params (DeltaSeconds :type "Float (single-precision)"))
  (`self.Camera Tick`))

(event `Disable After Time`
  (if (>= (`self.Time`) (`self.Wallrun Time`))
    (set `self.Time` 0.0))
  (`self.DelayedWhileLoop` (and (<= (`self.Time`) (`self.Wallrun Time`)) (`self.Is Wallrunning`))
    (:`Loop Body`
      (set `self.Time` (+ (`self.Time`) (`GameplayStatics.GetWorldDeltaSeconds`))))
    (:`Completed`
      (`self.Wallrun End`))))

(fn `Camera Tick`
  (bind _tilt_amount (`self.Tilt Amount`))
  (if (`self.Is Wallrunning`)
    (if (`self.Rightside`)
      (`self.Camera Tilt` (* _tilt_amount -1.0))
      (else
        (`self.Camera Tilt` _tilt_amount)))
    (else
      (`self.Camera Tilt` 0.0))))

(fn `Camera Tilt`
  (params (Tilt :type "Float (double-precision)"))
  (bind _returnvalue (`GameplayStatics.GetPlayerController` 0))
  (bind _returnvalue_2 (`Controller.GetControlRotation` _returnvalue))
  (`Controller.SetControlRotation` _returnvalue (`KismetMathLibrary.RInterpTo` _returnvalue_2 (`KismetMathLibrary.MakeRotator` Tilt (.pitch _returnvalue_2) (.yaw _returnvalue_2)) (`GameplayStatics.GetWorldDeltaSeconds`) 10.0)))

(fn `Disable Wallrun`
  (set `self.Wallrun Enabled` false)
  (`KismetSystemLibrary.K2_SetTimer` null "Enable Wallrun" (`self.Wallrun Delay`)))

(fn `Enable Wallrun`
  (`KismetSystemLibrary.K2_ClearTimer` null "Disable Wallrun")
  (set `self.Wallrun Enabled` true))

(fn `Wallrun End`
  (if (`self.Is Wallrunning`)
    (bind _output_get (set `self.Is Wallrunning` false))
    (set `self.Rightside` _output_get)
    (set `CharacterMovementComponent.GravityScale` (`self.DefaultGravity`) (`self.Movement Component`))
    (set `self.Time` 0.0)
    (`self.Disable Wallrun`)))

(fn `Wallrun Jump`
  (bind (_velocity_x _velocity_y) (`KismetMathLibrary.BreakVector` (`MovementComponent.Velocity` (`self.Movement Component`))))
  (bind (_returnvalue_x _returnvalue_y) (`KismetMathLibrary.BreakVector` (* (`KismetMathLibrary.Normal` (* (`KismetMathLibrary.Normal` (`self.Wallrun Normal`)) (1.0 1.0 0.0))) (`self.Wallrun Jump Speed`))))
  (if (`self.Is Wallrunning`)
    (`self.Wallrun End`)
    (`Character.LaunchCharacter` (`GameplayStatics.GetPlayerCharacter` 0) (`KismetMathLibrary.MakeVector` (+ _velocity_x _returnvalue_x) (+ _velocity_y _returnvalue_y) (`self.Wallrun Jump Height`)) false true)))

(fn `Wallrun Movement`
  (params (Start :type "Vector Structure") (End :type "Vector Structure") (`Wallrun Direction` :type "Float (double-precision)"))
  (returns (`On Wall` :type Boolean))
  (bind _returnvalue (`GameplayStatics.GetPlayerCharacter` 0))
  (bind (_velocity_x _velocity_y _velocity_z) (`KismetMathLibrary.BreakVector` (`MovementComponent.Velocity` (`self.Movement Component`))))
  (bind (_returnvalue_x _returnvalue_y) (`KismetMathLibrary.BreakVector` (* (`KismetMathLibrary.Cross_VectorVector` (`self.Wallrun Normal`) (0.0 0.0 1.0)) (* (`local.Wallrun Direction`) (`self.Wallrun Speed`)))))
  (bind _returnvalue_2 (`KismetMathLibrary.MakeVector` _returnvalue_x _returnvalue_y (`KismetMathLibrary.FInterpTo` _velocity_z 0.0 (`GameplayStatics.GetWorldDeltaSeconds`) 20.0)))
  (bind _outhit (`KismetSystemLibrary.LineTraceSingle` Start End "TraceTypeQuery1"))
  (bind (_bblockinghit _binitialoverlap _time _distance _location _impactpoint _normal) (`GameplayStatics.BreakHitResult` _outhit))
  (if _bblockinghit
    (bind (_in_range _out_vec) (`self.Valid Wallrun Surface` _normal))
    (if (and _in_range (`NavMovementComponent.IsFalling` (`self.Movement Component`)))
      (set `self.Wallrun Normal` _out_vec)
      (`Character.LaunchCharacter` _returnvalue (`self.Pull Player to Wall`) false false) ; Stick to Wall
      (if (`PlayerController.IsInputKeyDown` (`GameplayStatics.GetPlayerController` 0) "W")
        (`Character.LaunchCharacter` _returnvalue _returnvalue_2 true true) ; Move Player Forward
        (elif (`PlayerController.IsInputKeyDown` (`GameplayStatics.GetPlayerController` 0) "S")
          (`Character.LaunchCharacter` _returnvalue (* _returnvalue_2 (-1.0 -1.0 1.0)) true true) ; Move Player Backward
          (else
            (`Character.LaunchCharacter` _returnvalue (* _returnvalue_2 (0.0 0.0 1.0)) true true) ; Don't Move Player
          )))
      (`self.Disable After Time`)
      (return true)
      (else
        (return false)))
    (else
      (return false))))

(fn `Wallrun Update`
  (bind _movement_component (`self.Movement Component`))
  (if (`self.Wallrun Enabled`)
    (if (`PlayerController.IsInputKeyDown` (`GameplayStatics.GetPlayerController` 0) "D")
      (bind _on_wall (`self.Wallrun Movement` (`Actor.K2_GetActorLocation` (`GameplayStatics.GetPlayerCharacter` 0)) (`self.Wallrun End Vectors`) -1.0)) ; Right
      (if _on_wall
        (bind _output_get (set `self.Is Wallrunning` true))
        (set `self.Rightside` _output_get)
        (set `CharacterMovementComponent.GravityScale` (`KismetMathLibrary.FInterpTo` (`CharacterMovementComponent.GravityScale` _movement_component) (`self.TargetGravity`) (`GameplayStatics.GetWorldDeltaSeconds`) 10.0) _movement_component :!label _label)
        (else
          (if (`self.Rightside`) :!label _label_2
            _
            (elif (`PlayerController.IsInputKeyDown` (`GameplayStatics.GetPlayerController` 0) "A")
              (bind _on_wall_2 (`self.Wallrun Movement` (`Actor.K2_GetActorLocation` (`GameplayStatics.GetPlayerCharacter` 0)) (`.Left` (`self.Wallrun End Vectors`)) 1.0)) ; Left
              (if _on_wall_2
                (set `self.Is Wallrunning` true)
                (set `self.Rightside` false)
                (goto _label)
                (else
                  _))))
          (`self.Wallrun End`)))
      (else
        (goto _label_2)))))