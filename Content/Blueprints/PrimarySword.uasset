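; PrimarySword is a melee weapon Blueprint that performs the player's primary sword attack.
; On PrimaryAttack, if off cooldown, it plays a swing sound and sphere-traces forward from player 0 along its facing, using Range and Radius against PhysicsBody objects.
; A hit Enemy takes Damage through its EnemyHealth.
; A half-second retriggerable delay then resets the cooldown flag.
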(event `self.PrimaryAttack`
  (bind _returnvalue (`GameplayStatics.GetPlayerCharacter` 0))
  (bind _returnvalue_2 (`self.K2_GetActorLocation` _returnvalue))
  (if (`self.OffCooldown`)
    (`GameplayStatics.PlaySoundAtLocation` "/Game/SoundEffects/swing-6045.swing-6045" (`self.K2_GetActorLocation`) (struct) 3.0 1.0 -0.1 null null null null)
    (set `self.OffCooldown` false)
    (bind _outhit (`KismetSystemLibrary.SphereTraceSingleForObjects` _returnvalue_2 (+ _returnvalue_2 (* (`KismetMathLibrary.Conv_RotatorToVector` (`self.K2_GetActorRotation` _returnvalue)) (`self.Range`))) (`self.Radius`) (`|MakeArray` "ObjectTypeQuery4" :!type "EObjectTypeQuery Enum")))
    (bind _asenemy (cast `/Game/Blueprints/Enemy` (`.HitActor` (`GameplayStatics.BreakHitResult` _outhit)))
      (:`then`
        (`/Game/Blueprints/EnemyHealth.takeDamage` (`/Game/Blueprints/Enemy.EnemyHealth` _asenemy) (`self.Damage`)))
      (:`CastFailed`
        _))
    (`KismetSystemLibrary.RetriggerableDelay` 0.5)
    (set `self.OffCooldown` true)))

(fn `UserConstructionScript`
  (`parent.UserConstructionScript`))