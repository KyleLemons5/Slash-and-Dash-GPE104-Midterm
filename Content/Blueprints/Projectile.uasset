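; Projectile actor that damages the first-person player character when it overlaps it.
; It sets its life span on BeginPlay.
; On overlap with the player it applies damage through the character's PlayerHealth, plays an explosion sound and destroys itself.
; It passes through Enemy actors and is destroyed by any other overlap.
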(event `self.ReceiveBeginPlay`
  (`self.SetLifeSpan` (`self.Lifespan`)))

(event `self.ReceiveActorBeginOverlap`
  (params (OtherActor :type "Actor Object Reference"))
  (bind _asbp_first_person_character (cast `/Game/FirstPerson/Blueprints/BP_FirstPersonCharacter` OtherActor)
    (:`then`
      (`/Game/Blueprints/PlayerHealth.takeDamage` (`/Game/FirstPerson/Blueprints/BP_FirstPersonCharacter.PlayerHealth` _asbp_first_person_character) (`self.Damage`))
      (`GameplayStatics.PlaySoundAtLocation` "/Game/StarterContent/Audio/Explosion01.Explosion01" (`self.K2_GetActorLocation`) (struct) 0.7 1.0 0.0 null null null null)
      (`self.K2_DestroyActor`))
    (:`CastFailed`
      (cast `/Game/Blueprints/Enemy` OtherActor
        (:`CastFailed`
          (`self.K2_DestroyActor`))))))

(fn `UserConstructionScript`)