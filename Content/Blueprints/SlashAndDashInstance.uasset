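; SlashAndDashInstance holds the game's lives, score and weapon flag, and runs the flow between level start, death and victory.
; Start shows the title, moves every MovingWall, refreshes health and dash HUD, then triggers Spawners with index-staggered values.
; Death destroys the player, then reloads the level or shows GameOver when lives drop below zero.
; EndLevel opens Level2, or on Level2 shows the win screen and freezes time.
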(event `Death`
  (`GameplayStatics.PlaySoundAtLocation` "/Game/StarterContent/Audio/Collapse01.Collapse01" (`Actor.K2_GetActorLocation` (`GameplayStatics.GetPlayerCharacter` 0)) (struct) 1.0 1.0 0.0 null null null null)
  (`Actor.K2_DestroyActor` (`GameplayStatics.GetPlayerPawn` 0))
  (bind _returnvalue (`|CreateWidget` "/Game/UIStuff/Death.Death_C" (`GameplayStatics.GetPlayerController` 0)))
  (`UserWidget.AddToViewport` _returnvalue 0)
  (`KismetSystemLibrary.Delay` 3.0)
  (`Widget.SetVisibility` _returnvalue "Hidden")
  (set `self.Lives` (- (`self.Lives`) 1))
  (if (< (`self.Lives`) 0)
    (bind _returnvalue_2 (`|CreateWidget` "/Game/UIStuff/GameOver.GameOver_C" (`GameplayStatics.GetPlayerController` 0)))
    (`UserWidget.AddToViewport` _returnvalue_2 0)
    (set `PlayerController.bShowMouseCursor` true (`GameplayStatics.GetPlayerController` 0))
    (else
      (bind _returnvalue_3 (`GameplayStatics.GetCurrentLevelName` true))
      (`GameplayStatics.OpenLevel` (`KismetStringLibrary.Conv_StringToName` _returnvalue_3)))))

(event `Start`
  (bind _returnvalue (`|CreateWidget` "/Game/UIStuff/Title.Title_C" (`GameplayStatics.GetPlayerController` 0)))
  (`UserWidget.AddToViewport` _returnvalue 0)
  (bind _outactors (`GameplayStatics.GetAllActorsOfClass` "/Game/UIStuff/MovingWall.MovingWall_C"))
  (for _array_element _outactors
    (`/Game/UIStuff/MovingWall.MoveOverTime` _array_element))
  (set `self.HasWeapon` true)
  (`KismetSystemLibrary.Delay` 5.0)
  (`Widget.SetVisibility` _returnvalue "Hidden")
  (bind _asbp_first_person_character (cast `/Game/FirstPerson/Blueprints/BP_FirstPersonCharacter` (`GameplayStatics.GetPlayerCharacter` 0)))
  (`/Game/Blueprints/PlayerHealth.updateUI` (`/Game/FirstPerson/Blueprints/BP_FirstPersonCharacter.PlayerHealth` _asbp_first_person_character))
  (bind _dash (`/Game/FirstPerson/Blueprints/BP_FirstPersonCharacter.Dash` _asbp_first_person_character))
  (`/Game/UIStuff/DashHud.UpdateDashBar` (`/Game/Blueprints/Dash.DashHudCache` _dash) (`/Game/Blueprints/Dash.Dashes` _dash) (`/Game/Blueprints/Dash.DashChargeTime` _dash) (`/Game/Blueprints/Dash.ChargeTime` _dash))
  (bind _outactors_2 (`GameplayStatics.GetAllActorsOfClass` "/Game/Blueprints/Spawner.Spawner_C"))
  (for (_array_element_2 _array_index) _outactors_2
    (`/Game/Blueprints/Spawner.Spawn` _array_element_2 (/ (`KismetMathLibrary.Conv_IntToDouble` _array_index) 2.0))))

(event `Begin`
  (set `self.Lives` (`self.MaxLives`)))

(event `EndLevel`
  (bind _returnvalue (`GameplayStatics.GetPlayerController` 0))
  (bind _returnvalue_2 (`GameplayStatics.GetCurrentLevelName` true))
  (if (== _returnvalue_2 "Level2")
    (bind _returnvalue_3 (`|CreateWidget` "/Game/UIStuff/WinScreen.WinScreen_C" (`GameplayStatics.GetPlayerController` 0)))
    (`UserWidget.AddToViewport` _returnvalue_3 0)
    (bind _asbp_first_person_character (cast `/Game/FirstPerson/Blueprints/BP_FirstPersonCharacter` (`GameplayStatics.GetPlayerCharacter` 0)))
    (set `/Game/Blueprints/PlayerHealth.IsInvincible` true (`/Game/FirstPerson/Blueprints/BP_FirstPersonCharacter.PlayerHealth` _asbp_first_person_character))
    (`Actor.DisableInput` (`GameplayStatics.GetPlayerCharacter` 0) _returnvalue)
    (set `PlayerController.bShowMouseCursor` true _returnvalue)
    (`GameplayStatics.SetGlobalTimeDilation` 0.0)
    (else
      (`GameplayStatics.OpenLevel` "Level2"))))

(fn `AddPoints`
  (params (Points :type "Float (double-precision)"))
  (set `self.Score` (+ Points (`self.Score`))))

(fn `Reset`
  (set `self.Score` 0.0)
  (set `self.Lives` (`self.MaxLives`))
  (set `self.HasWeapon` false))